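; Game mode Blueprint for The Box that puts the in-game UI on screen when play begins.
; On BeginPlay it creates the WBP_TheBox widget, adds it to the viewport and keeps it as InGameUI.
; It then casts the active game mode to TheBoxGameMode, looks up a hardcoded clue by ID, and shows that clue's text and solution concatenated in the widget.
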(event EventBeginPlay
  (bind _returnvalue (UserInterface|CreateWidget "/Game/UI/WBP_TheBox.WBP_TheBox_C"))
  (UserInterface|Viewport|AddtoViewport _returnvalue 0)
  (bind _output_get (Variables|Default|SetInGameUI _returnvalue))
  (bind _asthe_box_game_mode (Utilities|Casting|CastToTheBoxGameMode (Game|GetGameMode)))
  (Class|InGameUI|SetText _output_get (Utilities|Text|ToText(String) (Utilities|String|Append (Utilities|String|ToString(Text) (.Clue (Utilities|Struct|BreakClues (Class|TheBoxGameMode|GetCluebyID _asthe_box_game_mode 3)))) (Utilities|String|ToString(Text) (.Solution (Utilities|Struct|BreakClues (Class|TheBoxGameMode|GetCluebyID _asthe_box_game_mode 3))))))))

(event EventTick
  (params (DeltaSeconds :type Float%20%28single-precision%29)))

(fn ConstructionScript)